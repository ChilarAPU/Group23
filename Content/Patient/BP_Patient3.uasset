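; BP_Patient3 is the third patient in a turn-based sequence of patient actors.
; At BeginPlay it finds BP_Patient1 and BP_Patient2, then checks both every Tick and sets its own PatientTurn once neither has the turn.
; Its LeaveRoom event sets Reverse and adds a Mini2 widget to the viewport.
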(event `self.ReceiveBeginPlay`
  (`parent.ReceiveBeginPlay`)
  (bind _returnvalue (`GameplayStatics.GetActorOfClass` "/Game/Patient/BP_Patient1.BP_Patient1_C"))
  (bind _returnvalue_2 (`GameplayStatics.GetActorOfClass` "/Game/Patient/BP_Patient2.BP_Patient2_C")))

(event `self.ReceiveTick`
  (params (DeltaSeconds :type "Float (single-precision)"))
  (`parent.ReceiveTick` DeltaSeconds)
  (if (not (or (`/Game/Patient/BP_PatientBase.PatientTurn` (stale `self.ReceiveBeginPlay` _returnvalue_2)) (`/Game/Patient/BP_PatientBase.PatientTurn` (stale `self.ReceiveBeginPlay` _returnvalue))))
    (set `self.PatientTurn` true)))

(event `self.LeaveRoom`
  (set `self.Reverse` true)
  (bind _returnvalue (`|CreateWidget` "/Game/Bradley/Mini2.Mini2_C"))
  (bind _output_get (set `self.NewVar_0` _returnvalue))
  (`UserWidget.AddToViewport` _output_get 0))

(fn `UserConstructionScript`
  (`parent.UserConstructionScript`))